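; BP_DoorTrigger is a one-shot trigger actor that reports its activation to a target door.
; The first overlap on its Box calls CountDoorTriggerMessage on TargetDoor and sets IsActived, so later overlaps are ignored; BeginPlay clears that flag.
; Activation also prints a debug message and swaps the static mesh's material to mark the trigger as used.
; The overlap does not filter which actor enters.
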(event `self.ReceiveBeginPlay`
  (set `self.IsActived` false))

(event `self.Box.OnComponentBeginOverlap`
  (params (OverlappedComponent :type "PrimitiveComponent Object Reference") (OtherActor :type "Actor Object Reference") (OtherComp :type "PrimitiveComponent Object Reference") (OtherBodyIndex :type Integer) (bFromSweep :type Boolean) (SweepResult :type "HitResult Structure (by ref)"))
  ; デバッグ用
  (if (not (`self.IsActived`))
    (`KismetSystemLibrary.PrintString` "Started!" true true (struct :`R` 1.0 :`B` 0.020854 :`A` 1.0))
    (message `/Game/ItoFolder/BP/Interface/BPI_DoorTrigger.CountDoorTrigger` (`self.TargetDoor`))
    (set `self.IsActived` true)
    (`PrimitiveComponent.SetMaterial` (`self.StaticMesh`) 0 "/Engine/EngineMaterials/EditorBrushMaterial.EditorBrushMaterial")))

(fn `UserConstructionScript`)