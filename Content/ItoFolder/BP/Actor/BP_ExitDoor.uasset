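; BP_ExitDoor is an exit door actor that swings open after its CountDoorTrigger event has been called four times.
; CountDoorTrigger increments a counter, and an IsOpened flag makes it ignore further calls once the door has opened.
; On the fourth call, OpenAnimation plays a timeline that lerps the whole actor's rotation from zero through a quarter turn, setting it absolutely.
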(event `self.ReceiveBeginPlay`
  (set `self.IsOpened` false)
  (set `self.CountTrigger` 0))

(event `/Game/ItoFolder/BP/Interface/BPI_DoorTrigger.CountDoorTrigger`
  ; すでに扉開いてるなら
  ; 処理しない
  (if (not (`self.IsOpened`))
    (set `self.CountTrigger` (+ (`self.CountTrigger`) 1))
    (if (== (`self.CountTrigger`) 4)
      (bind (_direction _alpha) (`Timeline|TL_OpenDoor`)
        (:`Update`
          (`self.K2_SetActorRotation` (`KismetMathLibrary.RLerp` (struct) (struct :`Yaw` -90.0) _alpha))
          (set `self.IsOpened` true))))))

(fn `UserConstructionScript`)